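; AnimatedAppearObject_BP is an actor with a configurable mesh that starts hidden in game and slides into place when Activate is called.
; Construction assigns the mesh and a dynamic instance of ReferenceMaterial with Opacity set to zero, which no graph here changes afterwards.
; Activate unhides the mesh and plays a timeline sized to AnimationTime, lerping relative location from StartPosition to EndPosition using the track value divided by AnimationTime.
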(event EventActivate
  (params (IsActivate :type Boolean))
  ;[1 1 1] Activation
  (Development|SetHiddeninGame (Variables|Default|GetStaticMesh) false false)
  (bind _lerp (Timeline|AnimationTimeline Play)
    (:Update
      (Transformation|SetRelativeLocation (Variables|Default|GetStaticMesh) (Math|Vector|Lerp(Vector) (Variables|Default|GetStartPosition) (Variables|Default|GetEndPosition) (/ _lerp (Variables|Default|GetAnimationTime))) false false))))

(event EventBeginPlay
  ;[1 1 1] Init
  (Components|Timeline|SetTimelineLength (Variables|Default|GetAnimationTimeline) (Variables|Default|GetAnimationTime))
  (Development|SetHiddeninGame (Variables|Default|GetStaticMesh) true false))

(fn ConstructionScript
  (bind _staticmesh (Variables|Default|GetStaticMesh))
  (Components|StaticMesh|SetStaticMesh _staticmesh (Variables|Default|GetMesh))
  (bind _returnvalue (Rendering|Material|CreateDynamicMaterialInstance (Variables|Default|GetReferenceMaterial) "None" "None" :!class /Script/Engine.KismetMaterialLibrary))
  (bind _output_get (Variables|Default|SetDynamicMaterial _returnvalue))
  (Rendering|Material|SetScalarParameterValue _output_get "Opacity" 0.0 :!class /Script/Engine.MaterialInstanceDynamic)
  (Rendering|Material|SetMaterial _staticmesh 0 _output_get))