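; Level-change trigger zone, a child Blueprint that switches levels when the player is inside the zone and looking at its target.
; Each Tick runs the parent logic, then checks the IsPlayerEnteredZone and IsLookingAt flags.
; While both are true, it calls SwitchLevel on FirstPersonGM_BP with NewLevelName, with no guard against repeat calls.
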(event EventBeginPlay
  (|CallParentFunction) ; This node is disabled and will not be called.\nDrag off pins to build functionality.
)

(event Collision|EventActorBeginOverlap
  (params (OtherActor :type Actor%20Object%20Reference)))

(event EventTick
  (params (DeltaSeconds :type Float%20%28single-precision%29))
  (|CallParentFunction DeltaSeconds)
  (if (and (Variables|Default|GetIsPlayerEnteredZone) (Variables|Default|GetIsLookingAt))
    (bind _asfirst_person_gm_bp (Utilities|Casting|CastToFirstPersonGM_BP (Game|GetGameMode)))
    (Default|SwitchLevel _asfirst_person_gm_bp (Variables|Default|GetNewLevelName))))

(fn ConstructionScript
  (|CallParentFunction))