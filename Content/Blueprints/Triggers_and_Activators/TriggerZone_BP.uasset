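; Trigger zone Blueprint that sends activate and deactivate messages to a target when actors overlap its box.
; An IsAllowedCheck gate passes only actors whose exact class is in AllowedObjects.
; Entering calls ActivateMessage with true on ActivationTarget, while leaving sends false only if ActivateOnExit is set.
; The construction script sizes the box from the Size variable.
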(event OnComponentEndOverlap(Box)
  (params (OverlappedComponent :type Primitive%20Component%20Object%20Reference) (OtherActor :type Actor%20Object%20Reference) (OtherComp :type Primitive%20Component%20Object%20Reference) (OtherBodyIndex :type Integer))
  (if (Variables|Default|GetActivateOnExit)
    (Utilities|IsAllowedCheck OtherActor)
    (Class|ICommunicationBP|Activate(Message) (Variables|Default|GetActivationTarget) false)))

(event OnComponentBeginOverlap(Box)
  (params (OverlappedComponent :type Primitive%20Component%20Object%20Reference) (OtherActor :type Actor%20Object%20Reference) (OtherComp :type Primitive%20Component%20Object%20Reference) (OtherBodyIndex :type Integer) (bFromSweep :type Boolean) (SweepResult :type Hit%20Result%20Structure%20%28by%20ref%29))
  (Utilities|IsAllowedCheck OtherActor)
  (Class|ICommunicationBP|Activate(Message) (Variables|Default|GetActivationTarget) true))

(fn ConstructionScript
  (Components|Box|SetBoxExtent (Variables|Default|GetBox) (Variables|Default|GetSize) true))