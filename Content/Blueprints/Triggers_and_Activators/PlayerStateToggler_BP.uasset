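; PlayerStateToggler_BP is a trigger volume that changes whether the player can jump.
; When a FirstPersonCharacterBP begins overlapping its Box, it writes NewCanJumping to the CanJumping flag of player pawn 0, with no reversal on exit.
; The construction script sizes the Box from the Size variable.
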(event OnComponentBeginOverlap(Box)
  (params (OverlappedComponent :type Primitive%20Component%20Object%20Reference) (OtherActor :type Actor%20Object%20Reference) (OtherComp :type Primitive%20Component%20Object%20Reference) (OtherBodyIndex :type Integer) (bFromSweep :type Boolean) (SweepResult :type Hit%20Result%20Structure%20%28by%20ref%29))
  (if (== (Utilities|GetClass OtherActor) "/Game/Blueprints/Player/FirstPersonCharacterBP.FirstPersonCharacterBP_C")
    (bind _asfirst_person_character_bp (Utilities|Casting|CastToFirstPersonCharacterBP (Game|Player|GetPlayerPawn 0)))
    (Variables|/Script/PuzzleGame.FirstPersonCharacter|SetCanJumping _asfirst_person_character_bp (Variables|Default|GetNewCanJumping))))

(fn ConstructionScript
  (Components|Box|SetBoxExtent (Variables|Default|GetBox) (Variables|Default|GetSize) true))