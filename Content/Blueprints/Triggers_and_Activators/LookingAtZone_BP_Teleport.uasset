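; Looking-at zone trigger that teleports the player to an exit point when they are inside the zone and looking at the target.
; Tick polls the inherited-style zone and gaze flags, then calls TeleportPlayer.
; The teleport mirrors the player's offset from the root at TeleportExit, reverses velocity, and adds CorrectiveRotation to control rotation.
; The construction script matches the ExitZone box to the trigger Box at TeleportExit.
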(event EventBeginPlay
  (|CallParentFunction))

(event EventTick
  (params (DeltaSeconds :type Float%20%28single-precision%29))
  (|CallParentFunction DeltaSeconds)
  (if (and (Variables|Default|GetIsPlayerEnteredZone) (Variables|Default|GetIsLookingAt))
    (CallFunction|TeleportPlayer)))

(fn ConstructionScript
  (|CallParentFunction)
  (Components|Box|SetBoxExtent (Variables|Default|GetExitZone) (Variables|/Script/Engine.BoxComponent|GetBoxExtent (Variables|Default|GetBox)) true)
  (Transformation|SetRelativeLocation (Variables|Default|GetExitZone) (Variables|Default|GetTeleportExit) false false))

(fn TeleportPlayer
  (bind _returnvalue (Game|GetPlayerController 0))
  (bind _correctiverotation (Variables|Default|GetCorrectiveRotation))
  (bind _player (Variables|Default|GetPlayer))
  (bind _returnvalue_2 (Pawn|GetControlRotation _returnvalue :!class /Script/Engine.Controller))
  (bind _charactermovement (Variables|/Script/Engine.Character|GetCharacterMovement _player))
  (Transformation|SetActorLocation (Variables|Default|GetPlayer) (+ (- (Transformation|GetWorldLocation (Variables|Default|GetDefaultSceneRoot)) (Transformation|GetActorLocation (Variables|Default|GetPlayer))) (+ (Transformation|GetActorLocation) (Variables|Default|GetTeleportExit))) false false)
  (Variables|/Script/Engine.MovementComponent|SetVelocity _charactermovement (* (Variables|/Script/Engine.MovementComponent|GetVelocity _charactermovement) -1.0))
  (Pawn|SetControlRotation _returnvalue (Math|Rotator|MakeRotator (+ (.roll _returnvalue_2) (.roll _correctiverotation)) (+ (.pitch _returnvalue_2) (.pitch _correctiverotation)) (+ (.yaw _returnvalue_2) (.yaw _correctiverotation)))))