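; Button_BP is an interactable toggle button that switches an assigned actor on and off.
; Interact plays or reverses a timeline, depending on IsActive, to slide the Cube a short distance along its local Y axis.
; When the timeline finishes, the button flips IsActive, sends the new state to ActorToActivate through ActivateMessage and plays an activation sound at its location.
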(event EventInteract
  (if (Variables|Default|GetIs%20Active)
    (bind _newtrack_0 (Timeline|Timeline_0 Reverse)
      (:Update
        (Transformation|SetRelativeLocation (Variables|Default|GetCube) (Math|Vector|Lerp(Vector) "0, 0, 0" "0.000000,10.000000,0.000000" _newtrack_0) false false))
      (:Finished
        (bind _output_get (Variables|Default|SetIs%20Active (not (Variables|Default|GetIs%20Active))))
        (Class|ICommunicationBP|Activate(Message) (Variables|Default|GetActor%20To%20Activate) _output_get)
        (Audio|PlaySoundatLocation (Variables|Default|GetActivation%20Sound) (Transformation|GetActorLocation) "0, 0, 0" 1.0 1.0 0.0 0 0 0)))
    (else
      (Timeline|Timeline_0 Play))))

(fn ConstructionScript)