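; Pressure-plate floor button that activates a linked actor while something overlaps its trigger box.
; A timeline slides the mesh between disabled and enabled positions, playing on overlap begin and reversing on overlap end.
; When movement finishes, its direction sets the active state, recolors the mesh through a new dynamic material instance, plays a sound, and passes the state to the target via ActivateMessage.
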(event OnComponentBeginOverlap(Box)
  (params (OverlappedComponent :type Primitive%20Component%20Object%20Reference) (OtherActor :type Actor%20Object%20Reference) (OtherComp :type Primitive%20Component%20Object%20Reference) (OtherBodyIndex :type Integer) (bFromSweep :type Boolean) (SweepResult :type Hit%20Result%20Structure%20%28by%20ref%29))
  (bind (_direction _lerp) (Timeline|ButtonMovement Play)
    (:Update
      (Transformation|SetRelativeLocation (Variables|Default|GetStaticMesh) (Math|Vector|Lerp(Vector) (Variables|Default|GetDisabledPosition) (Variables|Default|GetEnabledPosition) _lerp) false false))
    (:Finished
      (if (Utilities|Enum|Equal(Enum) _direction "Forward")
        (Variables|Default|SetIsActive true)
        (else
          (Variables|Default|SetIsActive false)))
      (CallFunction|ToggleColor (Variables|Default|GetEnabledColor) (Variables|Default|GetDisabledColor))
      (Audio|PlaySoundatLocation (Variables|Default|GetActivationSound) (Transformation|GetActorLocation) "0, 0, 0" 1.0 1.0 0.0 0 0 0)
      (Class|ICommunicationBP|Activate(Message) (Variables|Default|GetActor%20To%20Activate) (Variables|Default|GetIsActive)))))

(event OnComponentEndOverlap(Box)
  (params (OverlappedComponent :type Primitive%20Component%20Object%20Reference) (OtherActor :type Actor%20Object%20Reference) (OtherComp :type Primitive%20Component%20Object%20Reference) (OtherBodyIndex :type Integer))
  (bind (_direction _lerp) (Timeline|ButtonMovement Reverse)
    (:Update
      (Transformation|SetRelativeLocation (Variables|Default|GetStaticMesh) (Math|Vector|Lerp(Vector) (Variables|Default|GetDisabledPosition) (Variables|Default|GetEnabledPosition) _lerp) false false))
    (:Finished
      (if (Utilities|Enum|Equal(Enum) _direction "Forward")
        (Variables|Default|SetIsActive true)
        (else
          (Variables|Default|SetIsActive false)))
      (CallFunction|ToggleColor (Variables|Default|GetEnabledColor) (Variables|Default|GetDisabledColor))
      (Audio|PlaySoundatLocation (Variables|Default|GetActivationSound) (Transformation|GetActorLocation) "0, 0, 0" 1.0 1.0 0.0 0 0 0)
      (Class|ICommunicationBP|Activate(Message) (Variables|Default|GetActor%20To%20Activate) (Variables|Default|GetIsActive)))))

(event EventBeginPlay)

(event Collision|EventActorBeginOverlap
  (params (OtherActor :type Actor%20Object%20Reference)))

(fn ConstructionScript)

(fn ToggleColor
  (params (EnabledColor :type Linear%20Color%20Structure) (DisabledColor :type Linear%20Color%20Structure))
  (bind _staticmesh (Variables|Default|GetStaticMesh))
  (if (Variables|Default|GetIsActive)
    (bind _returnvalue (Rendering|Material|CreateDynamicMaterialInstance _staticmesh 0 "/Game/Materials/M_DevTexture_Master.M_DevTexture_Master" "None" :!class /Script/Engine.PrimitiveComponent))
    (Rendering|Material|SetVectorParameterValue _returnvalue "Color" EnabledColor :!class /Script/Engine.MaterialInstanceDynamic)
    (Rendering|Material|SetMaterial _staticmesh 0 _returnvalue)
    (else
      (bind _returnvalue_2 (Rendering|Material|CreateDynamicMaterialInstance _staticmesh 0 "/Game/Materials/M_DevTexture_Master.M_DevTexture_Master" "None" :!class /Script/Engine.PrimitiveComponent))
      (Rendering|Material|SetVectorParameterValue _returnvalue_2 "Color" DisabledColor :!class /Script/Engine.MaterialInstanceDynamic)
      (Rendering|Material|SetMaterial _staticmesh 0 _returnvalue_2))))