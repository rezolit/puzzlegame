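; Door actor that swings its static mesh between closed and opened rotations when it receives an Activate event with a new state.
; A timeline drives the rotation lerp, playing forward to open and in reverse to close, with a matching sound for each direction.
; Timeline progress also sets the start offset for the next sound, so audio stays in step when the door reverses mid-swing.
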(event EventActivate
  (params (IsActivate :type Boolean))
  (bind _audio (Variables|Default|GetAudio))
  (bind _audio_2 (Variables|Default|GetAudio))
  (if (Math|Boolean|NotEqual(Boolean) (Variables|Default|GetIsOpened) IsActivate)
    (bind _output_get (Variables|Default|SetIsOpened IsActivate))
    (Audio|Components|Audio|Stop (Variables|Default|GetAudio))
    (if _output_get
      (Audio|Components|Audio|SetSound _audio_2 (Variables|Default|GetOpenSound))
      (Audio|Components|Audio|Play _audio_2 (Variables|Default|GetCurrentAnimationTime))
      (bind _lerp (Timeline|Opening Play)
        (:Update
          (if (Variables|Default|GetIsOpened)
            (Variables|Default|SetCurrentAnimationTime (- 2.0 (* 2 _lerp)))
            (else
              (Variables|Default|SetCurrentAnimationTime (* 2 _lerp))))
          (Transformation|SetRelativeRotation (Variables|Default|GetStaticMesh) (Math|Rotator|Lerp(Rotator) (Variables|Default|GetClosedRotation) (Variables|Default|GetOpenedRotation) _lerp) false false)))
      (else
        (Audio|Components|Audio|SetSound _audio (Variables|Default|GetCloseSound))
        (Audio|Components|Audio|Play _audio (Variables|Default|GetCurrentAnimationTime))
        (Timeline|Opening Reverse)))))

(fn ConstructionScript)