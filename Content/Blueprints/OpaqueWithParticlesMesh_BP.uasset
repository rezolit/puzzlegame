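; Blueprint actor that drives a Niagara particle system built around a static mesh, with an on/off activation state.
; The construction script passes the Floor_400x400 mesh to the system's Particles.ReferenceMesh user variable.
; BeginPlay sets Niagara active from IsActive.
; The Activate event flips IsActive but sets the component from its own IsActivate argument, so flag and effect can diverge.
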(event EventActivate
  (params (IsActivate :type Boolean))
  (Variables|Default|SetIsActive (not (Variables|Default|GetIsActive)))
  (Components|Activation|SetActive (Variables|Default|GetNiagara) IsActivate false))

(event EventBeginPlay
  (Components|Activation|SetActive (Variables|Default|GetNiagara) (Variables|Default|GetIsActive) false))

(fn ConstructionScript
  (Class|NiagaraFunctionLibrary|OverrideSystemUserVariableStaticMesh (Variables|Default|GetNiagara) "Particles.ReferenceMesh" "/Game/StarterContent/Architecture/Floor_400x400.Floor_400x400"))