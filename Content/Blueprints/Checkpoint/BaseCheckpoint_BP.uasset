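; BaseCheckpoint_BP is a checkpoint trigger volume that activates when the first-person player character overlaps its box.
; The construction script sizes the box from the Size variable.
; On first overlap by FirstPersonCharacterBP, ActivateCheckpoint registers the checkpoint with FirstPersonGM_BP's activated checkpoint list and sets IsActive, so later overlaps are ignored.
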(event OnComponentBeginOverlap(Box)
  (params (OverlappedComponent :type Primitive%20Component%20Object%20Reference) (OtherActor :type Actor%20Object%20Reference) (OtherComp :type Primitive%20Component%20Object%20Reference) (OtherBodyIndex :type Integer) (bFromSweep :type Boolean) (SweepResult :type Hit%20Result%20Structure%20%28by%20ref%29))
  (if (not (Variables|Default|GetIsActive))
    (Utilities|Casting|CastToFirstPersonCharacterBP OtherActor)
    (CallFunction|ActivateCheckpoint)))

(fn ConstructionScript
  (Components|Box|SetBoxExtent (Variables|Default|GetBox) (Variables|Default|GetSize) true))

(fn ActivateCheckpoint
  ;[1 1 1] Add To Activated Checkpoints List
  (bind _asfirst_person_gm_bp (Utilities|Casting|CastToFirstPersonGM_BP (Game|GetGameMode)))
  (Default|AddNewActivatedCheckpoint _asfirst_person_gm_bp self)
  (Variables|Default|SetIsActive true))