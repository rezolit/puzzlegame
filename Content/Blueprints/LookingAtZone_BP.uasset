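; LookingAtZone_BP is a box zone that tracks whether the player, while inside it, is looking at a target.
; Begin and end overlaps with the FirstPersonCharacterBP toggle an inside flag.
; While that flag is set, Tick stores the result of the player's IsLookingAt check on LookAtTarget, which is not reset on exit.
; The construction script sizes the box from ZoneSize.
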(event OnComponentBeginOverlap(Box)
  (params (OverlappedComponent :type Primitive%20Component%20Object%20Reference) (OtherActor :type Actor%20Object%20Reference) (OtherComp :type Primitive%20Component%20Object%20Reference) (OtherBodyIndex :type Integer) (bFromSweep :type Boolean) (SweepResult :type Hit%20Result%20Structure%20%28by%20ref%29))
  (Utilities|Casting|CastToFirstPersonCharacterBP OtherActor)
  (Variables|Default|SetIsPlayerEnteredZone true))

(event OnComponentEndOverlap(Box)
  (params (OverlappedComponent :type Primitive%20Component%20Object%20Reference) (OtherActor :type Actor%20Object%20Reference) (OtherComp :type Primitive%20Component%20Object%20Reference) (OtherBodyIndex :type Integer))
  (Utilities|Casting|CastToFirstPersonCharacterBP OtherActor)
  (Variables|Default|SetIsPlayerEnteredZone false))

(event EventTick
  (params (DeltaSeconds :type Float%20%28single-precision%29))
  (if (Variables|Default|GetIsPlayerEnteredZone)
    (bind _result (Default|IsLookingat (Variables|Default|GetPlayer) (Variables|Default|GetLookAtTarget)))
    (Variables|Default|SetIsLookingAt _result)))

(event EventBeginPlay
  (bind _asfirst_person_character_bp (Utilities|Casting|CastToFirstPersonCharacterBP (Game|Player|GetPlayerPawn 0)))
  (Variables|Default|SetPlayer _asfirst_person_character_bp))

(fn ConstructionScript
  (Components|Box|SetBoxExtent (Variables|Default|GetBox) (Variables|Default|GetZone%20Size) true))