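; One-shot spike trap that, after an actor overlaps its trigger, waits a delay, then animates its spikes and damages actors touching them.
; BeginPlay builds a grid of scaled static mesh spikes from the spacing value and sizes a disabled BlockVolume to the trigger.
; A timeline lerps the spikes and an offset DeathZone together along Z, with a sound at the start.
; DeathZone overlaps apply damage, and BlockVolume switches to query-only collision when the animation finishes.
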(event OnComponentBeginOverlap(Trigger)
  (params (OverlappedComponent :type Primitive%20Component%20Object%20Reference) (OtherActor :type Actor%20Object%20Reference) (OtherComp :type Primitive%20Component%20Object%20Reference) (OtherBodyIndex :type Integer) (bFromSweep :type Boolean) (SweepResult :type Hit%20Result%20Structure%20%28by%20ref%29))
  (bind _deathzone (Variables|Default|GetDeathZone))
  (bind _relativelocation (Variables|/Script/Engine.SceneComponent|GetRelativeLocation _deathzone))
  ;[1 0.1864 0.3671] Activating trap
  (Collision|SetCollisionEnabled (Variables|Default|GetTrigger) "NoCollision")
  (Utilities|FlowControl|Delay (Variables|Default|GetActivationDelay))
  (Audio|PlaySoundatLocation (Variables|Default|GetActivatingSound) (Transformation|GetActorLocation) "0, 0, 0" 1.0 1.0 0.0 "/Game/Sounds/FP_Attenuation.FP_Attenuation" 0 0)
  (bind _lerp (Timeline|Spikes%20Animation Play)
    (:Update
      (for _array_element (Variables|Default|GetSpikes)
        (Transformation|SetRelativeLocation _array_element (Math|Vector|MakeVector (.x (Variables|/Script/Engine.SceneComponent|GetRelativeLocation _array_element)) (.y (Variables|/Script/Engine.SceneComponent|GetRelativeLocation _array_element)) (.z (Math|Vector|Lerp(Vector) (Math|Vector|MakeVector 0.0 0.0 (.z (Variables|Default|GetStartSpikesLocation))) (Math|Vector|MakeVector 0.0 0.0 (.z (Variables|Default|GetEndSpikesLocation))) _lerp))) false false))
      (Transformation|SetRelativeLocation _deathzone (Math|Vector|MakeVector (.x _relativelocation) (.y _relativelocation) (+ (.z (Math|Vector|Lerp(Vector) (Math|Vector|MakeVector 0.0 0.0 (.z (Variables|Default|GetStartSpikesLocation))) (Math|Vector|MakeVector 0.0 0.0 (.z (Variables|Default|GetEndSpikesLocation))) _lerp)) (Variables|Default|GetDeathZoneZOffset))) false false))
    (:Finished
      (Collision|SetCollisionEnabled (Variables|Default|Getblock%20volume) "QueryOnly"))))

(event OnComponentBeginOverlap(DeathZone)
  (params (OverlappedComponent :type Primitive%20Component%20Object%20Reference) (OtherActor :type Actor%20Object%20Reference) (OtherComp :type Primitive%20Component%20Object%20Reference) (OtherBodyIndex :type Integer) (bFromSweep :type Boolean) (SweepResult :type Hit%20Result%20Structure%20%28by%20ref%29))
  ;[0.03748 1 0.007351] Damage
  (Game|Damage|ApplyDamage OtherActor 1.0 0 0))

(event EventBeginPlay
  (bind _returnvalue (Math|Vector|MakeVector 0.0 0.0 0.0))
  (bind _block_volume (Variables|Default|Getblock%20volume))
  (bind _spikes_distance (Variables|Default|GetSpikes%20Distance))
  (bind _spikes_distance_2 (Variables|Default|GetSpikes%20Distance))
  (bind _returnvalue_2 (/ 4e+02 _spikes_distance_2))
  (bind _returnvalue_3 (Math|Float|Truncate _returnvalue_2))
  (bind _returnvalue_4 (- _returnvalue_3 1))
  ;[0.2238 0.3544 1] Init
  (for _index (range 1 _returnvalue_4)
    (for _index_2 (range 1 _returnvalue_4)
      (bind _returnvalue_5 (AddComponent|AddStaticMeshComponent false (Math|Transform|MakeTransform (Math|Vector|MakeVector (* _index (+ (.x _returnvalue) _spikes_distance)) (* _index_2 (+ (.y _returnvalue) _spikes_distance)) (.z (Variables|Default|GetStartSpikesLocation))) "0, 0, 0" "0.100000,0.100000,1.000000")))
      (Utilities|Array|Add (Variables|Default|GetSpikes) _returnvalue_5)
      (Rendering|Material|SetMaterial _returnvalue_5 0 "/Game/StarterContent/Materials/M_Metal_Burnished_Steel.M_Metal_Burnished_Steel")))
  (Components|Box|SetBoxExtent _block_volume (Variables|/Script/Engine.BoxComponent|GetBoxExtent (Variables|Default|GetTrigger)) true)
  (Collision|SetCollisionEnabled _block_volume "NoCollision"))

(fn ConstructionScript)